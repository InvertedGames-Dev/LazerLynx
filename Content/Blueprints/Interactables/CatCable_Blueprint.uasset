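; Interactable cable that hooks onto a BP_Lynx's CableSocket on overlap and later tethers the player to it.
; As the Lynx moves away, spool actors are destroyed in stages until the final cable length frees the far end from its anchor.
; The player then auto-attaches when near the cable component.
; Tick checks the tether distance, using a timeline lerp to drag the player horizontally back when near the limit.
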(event OnComponentBeginOverlap(Overlap)
  (params (OverlappedComponent :type Primitive%20Component%20Object%20Reference) (OtherActor :type Actor%20Object%20Reference) (OtherComp :type Primitive%20Component%20Object%20Reference) (OtherBodyIndex :type Integer) (bFromSweep :type Boolean) (SweepResult :type Hit%20Result%20Structure%20%28by%20ref%29))
  (bind _asbp_lynx (Utilities|Casting|CastToBP_Lynx OtherActor))
  (Transformation|AttachComponentToComponent self (Variables|/Script/Engine.Character|GetMesh _asbp_lynx) "CableSocket" "SnapToTarget" "SnapToTarget" "KeepWorld" true)
  (Variables|Default|SetLynx _asbp_lynx)
  (Actor|Tick|SetActorTickEnabled true))

(event EventBeginPlay
  (bind _cablecomponent (Variables|Default|GetCableComponent))
  (Variables|/Script/CableComponent.CableComponent|SetbAttachEnd _cablecomponent true)
  (Class|CableComponent|SetAttachEndto _cablecomponent (Variables|Default|GetAttach) "None" "None")
  (bind _asfirst_person_character (Utilities|Casting|CastToFirstPersonCharacter (Game|GetPlayerCharacter 0)))
  (Variables|Default|SetMyCharacter _asfirst_person_character))

(event EventTick
  (params (DeltaSeconds :type Float%20%28single-precision%29))
  (bind _cablecomponent (Variables|Default|GetCableComponent))
  (bind _mycharacter (Variables|Default|GetMyCharacter))
  (bind _cablecomponent_2 (Variables|Default|GetCableComponent))
  (bind _lynx (Variables|Default|GetLynx))
  (bind _cablespool (Variables|Default|GetCableSpool))
  (bind _cablefinaldistance (Variables|Default|GetCableFinalDistance))
  (bind _cablespool_2 (Variables|Default|GetCableSpool))
  (bind _cablecomponent_3 (Variables|Default|GetCableComponent))
  (bind _returnvalue (Transformation|GetWorldLocation _cablecomponent))
  (bind _returnvalue_2 (Transformation|GetActorLocation _mycharacter))
  (bind _output (Utilities|Array|Get(acopy) _cablespool_2))
  (bind _returnvalue_3 (Math|Vector|Distance(Vector) _returnvalue _returnvalue_2))
  (bind _returnvalue_4 (Transformation|GetDistanceTo _lynx _output))
  (if (Variables|Default|GetAttached)
    (if (Variables|Default|GetPlayerAttached)
      (if (> _returnvalue_3 (- (Variables|Default|GetCableFinalDistance) 1e+02))
        (Variables|Default|SetMoveTo _returnvalue_2)
        (bind _newtrack_0 (Timeline|Move PlayFromStart)
          (:Update
            (Transformation|SetActorLocation (Variables|Default|GetMyCharacter) (Math|Vector|MakeVector (.x (Math|Vector|Lerp(Vector) (Variables|Default|GetMoveTo) _returnvalue (* _newtrack_0 0.2))) (.y (Math|Vector|Lerp(Vector) (Variables|Default|GetMoveTo) _returnvalue (* _newtrack_0 0.2))) (.Z (Math|Vector|BreakVector (Variables|Default|GetMoveTo)))) false false))))
      (elif (< _returnvalue_3 2e+02)
        (Variables|/Script/CableComponent.CableComponent|SetbAttachEnd _cablecomponent_2 true)
        (Class|CableComponent|SetAttachEndto _cablecomponent_2 (Variables|Default|GetMyCharacter) "None" "None")
        (Variables|Default|SetPlayerAttached true)))
    (elif (> _returnvalue_4 _cablefinaldistance)
      (Variables|Default|SetAttached true)
      (Variables|/Script/CableComponent.CableComponent|SetbAttachEnd _cablecomponent_3 false)
      (Variables|/Script/CableComponent.CableComponent|SetCableLength _cablecomponent_3 (Variables|Default|GetCableFinalDistance))
      (for _array_element (Variables|Default|GetCableSpool)
        (Utilities|IsValid _array_element
          (:Is%20Valid
            (Actor|DestroyActor _array_element))))
      (elif (> _returnvalue_4 (* (/ _cablefinaldistance 4.0) (Variables|Default|GetUnspooled)))
        (Actor|DestroyActor (Utilities|Array|Get(acopy) _cablespool))
        (Utilities|Array|RemoveIndex _cablespool)
        (Math|Float|IncrementFloat (Variables|Default|GetUnspooled))))))

(fn ConstructionScript)