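; Interactable balloon that bobs in place and pops after being pointed at enough times.
; On BeginPlay it starts the Bob timeline at a random time to vary the phase, lerping slightly above its start location and replaying on finish.
; Each Pointedat event raises a Heat counter; at the threshold it plays a weapon fire sound once and destroys itself.
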(event EventBeginPlay
  (Variables|Default|SetStartLoc (Transformation|GetActorLocation))
  (Utilities|FlowControl|Sequence
    (:then_0
      (bind _updown (Timeline|Bob SetNewTime)
        (:Update
          (Transformation|SetActorLocation (Math|Vector|Lerp(Vector) (Variables|Default|GetStartLoc) (Math|Vector|MakeVector (.x (Variables|Default|GetStartLoc)) (.y (Variables|Default|GetStartLoc)) (+ (.z (Variables|Default|GetStartLoc)) 7.0)) _updown) false false))
        (:Finished
          (Utilities|FlowControl|Delay 0.001)
          (Timeline|Bob PlayFromStart))))
    (:then_1
      (Timeline|Bob Play))))

(event Collision|EventActorBeginOverlap
  (params (OtherActor :type Actor%20Object%20Reference)))

(event EventTick
  (params (DeltaSeconds :type Float%20%28single-precision%29)))

(event EventPointedat
  (bind _result (Math|Float|IncrementFloat (Variables|Default|GetHeat))
    (:%20%20
      (if (>= _result 1e+02)
        (Utilities|FlowControl|DoOnce false
          (:Completed
            (Audio|PlaySoundatLocation "/Game/Blueprints/FirstPerson/Audio/FirstPersonTemplateWeaponFire02.FirstPersonTemplateWeaponFire02" (Transformation|GetActorLocation) "0, 0, 0" 1.0 1.0 0.0 0 0 0)
            (Actor|DestroyActor)))))))

(fn ConstructionScript)