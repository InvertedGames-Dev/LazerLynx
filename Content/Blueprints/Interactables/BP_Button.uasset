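; BP_Button is an interactable floor button that activates a list of linked actors when walked over.
; Stepping on it plays a timeline that moves the Pressable component in Z and fires ButtonPressed from an Activate event track.
; ToggleButton lets it replay on every step, while otherwise a DoOnce limits it to one press.
; ButtonPressed sends ActivatedMessage to each of the ActivatedActors with an alternating FlipFlop state.
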(event Custom|Button%20Pressed
  (bind _isa (Utilities|FlowControl|FlipFlop)
    (:A
      _)
    (:B
      _))
  (for _array_element (Variables|Default|GetActivatedActors)
    (Class|InteractInterface|Activated(Message) _array_element _isa)))

(event EventWalkedOver
  (params (On :type Boolean))
  (if On
    (if (Variables|Default|GetToggle%20button)
      (bind _z (Timeline|Timeline_0 PlayFromStart)
        (:Update
          (Transformation|SetRelativeLocation (Variables|Default|GetPressable) (Math|Vector|MakeVector 0.0 0.0 _z) false false))
        (:Activate
          (CallFunction|ButtonPressed)))
      (else
        (Utilities|FlowControl|DoOnce false
          (:Completed
            (Timeline|Timeline_0 PlayFromStart)))))))

(fn ConstructionScript)