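; BP_LaserPoint is a laser point actor that detects when it is being shaken in place.
; Each tick, moving farther than ShakeSpeed since the last frame refreshes a cooldown, and the location enters a 61-slot ring buffer.
; LaserShake is true while the cooldown runs and the point stays within half of ShakeRadius of the buffer's average, separating shaking from travel.
; A Debug flag draws a sphere at that average.
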(event EventTick
  (params (DeltaSeconds :type Float%20%28single-precision%29))
  (bind _returnvalue (Transformation|GetActorLocation))
  (bind _shake_radius (Variables|Adjustments|GetShake%20Radius))
  (bind _vector_array_index (Variables|Default|GetVector%20Array%20index))
  (bind _vector_array (Variables|Default|GetVector%20Array))
  (bind _returnvalue_2 (Math|Vector|GetVectorArrayAverage _vector_array))
  (Utilities|FlowControl|Gate true
    (:Exit
      (if (> (Math|Vector|Distance(Vector) (Transformation|GetActorLocation) (Variables|Default|GetPrevious%20location)) (Variables|Adjustments|GetShake%20Speed))
        (Variables|Default|SetShake%20cooldown (+ (Utilities|Time|GetGameTimeinSeconds) (Variables|Adjustments|GetShake%20Cooldown%20Time))))
      (Variables|Default|SetPrevious%20location _returnvalue)
      (Utilities|Array|SetArrayElem (Variables|Default|GetVector%20Array) _vector_array_index _returnvalue true)
      (if (== _vector_array_index 60)
        (|SetBy-RefVar _vector_array_index)
        (else
          (Math|Integer|IncrementInt _vector_array_index
            (:%20%20
              _))))
      (if (Variables|Default|GetDebug)
        (Rendering|Debug|DrawDebugSphere _returnvalue_2 _shake_radius 12 "(R=1.000000,G=0.000000,B=0.000000,A=1.000000)" 0.0 1.0))
      (Variables|Default|SetLaser%20Shake (and (< (Math|Vector|Distance(Vector) _returnvalue_2 (Transformation|GetActorLocation)) (/ _shake_radius 2.0)) (> (Variables|Default|GetShake%20cooldown) (Utilities|Time|GetGameTimeinSeconds)))))))

(event EventBeginPlay
  (bind _returnvalue (Transformation|GetActorLocation))
  (bind _returnvalue_2 (Transformation|GetActorLocation))
  (bind _shake_radius (Variables|Adjustments|GetShake%20Radius))
  (bind _vector_array_index (Variables|Default|GetVector%20Array%20index))
  (bind _vector_array (Variables|Default|GetVector%20Array))
  (bind _returnvalue_3 (Math|Vector|GetVectorArrayAverage _vector_array))
  (Variables|Default|SetPrevious%20location _returnvalue_2)
  (Utilities|FlowControl|Gate true) ; enters at Open
)

(fn ConstructionScript)