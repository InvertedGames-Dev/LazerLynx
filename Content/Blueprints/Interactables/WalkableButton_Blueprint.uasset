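; Walkable floor button that sinks when stepped on and switches a list of target actors on or off.
; WalkedOver stores the pressed state, then plays the ButtonUp timeline to lower Pressable, or reverses it after a short delay.
; When the timeline finishes, it sends ActivatedMessage to each of ActivatedActors, deriving the on/off value from playback direction.
; A check against repeated identical states exists but is not connected.
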(event EventBeginPlay
  (Variables|Default|SetStartPos (Variables|/Script/Engine.SceneComponent|GetRelativeLocation (Variables|Default|GetPressable))))

(event EventWalkedOver
  (params (On :type Boolean))
  (bind _startpos (Variables|Default|GetStartPos))
  (bind (_x _y _z) (Math|Vector|BreakVector _startpos))
  (Variables|Default|SetPressed On)
  (if On
    (bind (_direction _newtrack_0) (Timeline|ButtonUp PlayFromStart)
      (:Update
        (Transformation|SetRelativeLocation (Variables|Default|GetPressable) (Math|Vector|Lerp(Vector) _startpos (Math|Vector|MakeVector _x _y (- _z 2e+01)) _newtrack_0) false false))
      (:Finished
        (for _array_element (Variables|Default|GetActivatedActors)
          (Class|InteractInterface|Activated(Message) _array_element (Utilities|Select :Index _direction :Forward true :Backward false)))))
    (else
      (Utilities|FlowControl|Delay 0.5)
      (Timeline|ButtonUp ReverseFromEnd))))

(fn ConstructionScript)