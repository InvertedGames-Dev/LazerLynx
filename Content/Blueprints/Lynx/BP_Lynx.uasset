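; BP_Lynx is the AI-controlled lynx character, which reacts to a laser and notifies actors it lands on or walks over.
; Each tick it eases LookArrow toward LookAtLocation while the controller's blackboard reports the laser visible, otherwise back to a resting rotation.
; A forward line trace, scaled by velocity, makes it jump when it hits a specific object type.
; Landing and WalkedOverCollision overlaps send messages to the other actor.
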(event OnComponentBeginOverlap(WalkedOverCollision)
  (params (OverlappedComponent :type Primitive%20Component%20Object%20Reference) (OtherActor :type Actor%20Object%20Reference) (OtherComp :type Primitive%20Component%20Object%20Reference) (OtherBodyIndex :type Integer) (bFromSweep :type Boolean) (SweepResult :type Hit%20Result%20Structure%20%28by%20ref%29))
  ;[1 1 1] Interactions
  (Class|InteractInterface|WalkedOver(Message) OtherActor true))

(event OnComponentEndOverlap(WalkedOverCollision)
  (params (OverlappedComponent :type Primitive%20Component%20Object%20Reference) (OtherActor :type Actor%20Object%20Reference) (OtherComp :type Primitive%20Component%20Object%20Reference) (OtherBodyIndex :type Integer))
  ;[1 1 1] Interactions
  (Class|InteractInterface|WalkedOver(Message) OtherActor false))

(event EventOnLanded
  (params (Hit :type Hit%20Result%20Structure%20%28by%20ref%29))
  ;[1 1 1] Interactions
  (Class|InteractInterface|Landedon(Message) (.HitActor (Collision|BreakHitResult Hit))))

(event EventTick
  (params (DeltaSeconds :type Float%20%28single-precision%29))
  (bind _returnvalue (Transformation|GetActorLocation))
  (CallFunction|SetLookRotation)
  (Variables|Default|SetNeck%20Location (Transformation|GetSocketLocation (Variables|Character|GetMesh) "Neck"))
  (bind _returnvalue_2 (Collision|LineTraceForObjects _returnvalue (Utilities|DirectionalTrace _returnvalue (Transformation|GetActorForwardVector) (/ (Math|Vector|VectorLength (Transformation|GetVelocity)) 3.0)) (Utilities|Array|MakeArray "ObjectTypeQuery9") false 0 "None"))
  (if _returnvalue_2
    (Character|Jump)))

(fn ConstructionScript)

(fn SetLookRotation
  (bind _look_arrow (Variables|Default|GetLook%20arrow))
  (bind _asai_lynx_controller (Utilities|Casting|CastToAI_LynxController (AI|GetAIController self)))
  (if (ScalableFloat|GetValueasBool (AI|GetBlackboard _asai_lynx_controller) (Utilities|Name|MakeLiteralName "Laser Visible"))
    (Transformation|SetWorldRotation _look_arrow (Math|Interpolation|RInterpTo (Transformation|GetWorldRotation _look_arrow) (Math|Rotator|FindLookatRotation (Transformation|GetWorldLocation _look_arrow) (Variables|Default|GetLook%20at%20location)) (Utilities|Time|GetWorldDeltaSeconds) 5.0) false false)
    (else
      (Transformation|SetRelativeRotation _look_arrow (Math|Interpolation|RInterpTo (Variables|/Script/Engine.SceneComponent|GetRelativeRotation _look_arrow) "0,90.000000, 0" (Utilities|Time|GetWorldDeltaSeconds) 5.0) false false))))