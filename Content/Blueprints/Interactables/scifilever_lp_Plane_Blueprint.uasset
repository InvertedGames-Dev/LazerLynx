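; Sci-fi lever that triggers an airlock losing ending when the BP_Lynx character overlaps its box.
; A timeline swings the lever, then the Lynx's AI controller gets a scared event and a sound plays.
; A second timeline rotates the airlock door, drags FPC away and switches the light color between white and red.
; It then calls a loss on FPC and unlocks the Spacewalk achievement.
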(event OnComponentBeginOverlap(Box)
  (params (OverlappedComponent :type Primitive%20Component%20Object%20Reference) (OtherActor :type Actor%20Object%20Reference) (OtherComp :type Primitive%20Component%20Object%20Reference) (OtherBodyIndex :type Integer) (bFromSweep :type Boolean) (SweepResult :type Hit%20Result%20Structure%20%28by%20ref%29))
  (bind _rotation (Variables|Default|GetRotation))
  (bind _location (Variables|Default|GetLocation))
  (bind _asbp_lynx (Utilities|Casting|CastToBP_Lynx OtherActor))
  (bind _lever (Timeline|Pulled Play)
    (:Update
      (Transformation|SetRelativeRotation (Variables|Default|GetScene) (Math|Rotator|Lerp(Rotator) "-20.000000,0.000000,0.000000" "-110.000000,0.000000, 0" _lever) false false))
    (:Finished
      (Utilities|FlowControl|Delay 0.2)
      (bind _asai_lynx_controller (Utilities|Casting|CastToAI_LynxController (AI|GetAIController _asbp_lynx)))
      (Default|EventScared _asai_lynx_controller)
      (Audio|PlaySoundatLocation "/Game/Blueprints/FirstPerson/Audio/FirstPersonTemplateWeaponFire02.FirstPersonTemplateWeaponFire02" "0, 0,150.000000" "0, 0, 0" 1.0 1.0 0.0 0 0 0)
      (bind (_direction _door _character _light) (Timeline|Airlocked Play)
        (:Update
          (Transformation|SetActorRotation (Variables|Default|GetAirlockDoor) (Math|Rotator|Lerp(Rotator) (Variables|Default|GetRotation) (Math|Rotator|MakeRotator (.roll _rotation) (.pitch _rotation) (+ (.yaw _rotation) 1e+02)) _door))
          (Transformation|SetActorLocation (Variables|Default|GetFPC) (Math|Vector|Lerp(Vector) _location (- _location "1200.000000, 0,60.000000") _character) false false)
          (Rendering|Components|Light|SetLightColor (Variables|/Script/Engine.Light|GetLightComponent (Variables|Default|GetLight)) (Utilities|Select :Index (Math|Float|Truncate _light) :Option%200 "(R=1.000000,G=1.000000,B=1.000000,A=1.000000)" :Option%201 "(R=1.000000,G=0.004520,B=0.000000,A=1.000000)") true))
        (:Finished
          (Utilities|FlowControl|Delay 1.0)
          (Default|WinorLose (Variables|Default|GetFPC) false 1)
          (bind _asmy_game_instance (Utilities|Casting|CastToMyGameInstance (Game|GetGameInstance)))
          (Default|UnlockAch _asmy_game_instance "Spacewalk"))))))

(event EventBeginPlay
  (Variables|Default|SetRotation (Transformation|GetActorRotation (Variables|Default|GetAirlockDoor)))
  (Variables|Default|SetLocation (Transformation|GetActorLocation (Variables|Default|GetFPC))))

(fn ConstructionScript)