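; MyGameInstance holds the game's achievement list and marks entries as unlocked.
; Its BeginPlay event copies every row of the AchivementsTable data table into the Achievements array.
; UnlockAch searches that array by name and rewrites each matching entry with the unlocked flag set, keeping its name, description and picture.
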(event Custom|BeginPlay
  (bind _outrownames (DataTable|GetDataTableRowNames "/Game/Blueprints/UI/AchivementsTable.AchivementsTable"))
  (for _array_element _outrownames
    (bind _returnvalue (Utilities|GetDataTableRow "/Game/Blueprints/UI/AchivementsTable.AchivementsTable" _array_element)
      (:then
        (Utilities|Array|Add (Variables|Default|GetAchievements) _returnvalue)))))

(event Custom|UnlockAch
  (params (Name :type String))
  (bind _achievements (Variables|Default|GetAchievements))
  (for (_array_element _array_index) _achievements
    (if (Utilities|Enum|Equal(Enum) Name (.Name (Utilities|Struct|BreakAchievement _array_element)))
      (Utilities|Array|SetArrayElem _achievements _array_index (Utilities|Struct|MakeAchievement (.Name (Utilities|Struct|BreakAchievement _array_element)) (.Description (Utilities|Struct|BreakAchievement _array_element)) (.Picture (Utilities|Struct|BreakAchievement _array_element)) true)))))